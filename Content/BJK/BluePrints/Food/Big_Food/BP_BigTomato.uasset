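; BP_BigTomato is a big tomato food actor that the player cuts into BP_Tomato pieces with a gripped knife.
; A box overlap with a gripped BP_Knife counts a cut, swaps the mesh to a slice and spawns a piece at the mesh location.
; A flag blocks further cuts until half a second after an overlap ends, and the second cut destroys the actor.
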(event OnComponentBeginOverlap(Box)
  (params (OverlappedComponent :type Primitive%20Component%20Object%20Reference) (OtherActor :type Actor%20Object%20Reference) (OtherComp :type Primitive%20Component%20Object%20Reference) (OtherBodyIndex :type Integer) (bFromSweep :type Boolean) (SweepResult :type Hit%20Result%20Structure%20%28by%20ref%29))
  (bind _staticmesh (Variables|Default|GetStaticMesh))
  (bind _returnvalue (Transformation|GetWorldLocation _staticmesh))
  (bind _asbp_knife (Utilities|Casting|CastToBP_Knife OtherActor))
  (if (and (Variables|/Game/BJK/BluePrints/cuttingboard/BP_Knife.BP_Knife_C|GetGripKnife _asbp_knife) (Variables|Default|GetDelay))
    (Variables|Default|SetCut (+ (Variables|Default|GetCut) 1))
    (Variables|Default|SetDelay false)
    (Components|StaticMesh|SetStaticMesh (Variables|Default|GetStaticMesh) "/Game/BJK/BluePrints/Food/Big_Food/tom_slice.tom_slice")
    (Game|SpawnActorfromClass "/Game/BJK/BluePrints/Food/BP_Tomato.BP_Tomato_C" (Math|Transform|MakeTransform (Math|Vector|MakeVector (.x _returnvalue) (.y _returnvalue) (.z _returnvalue)) "0, 0, 0" "1.000000,1.000000,1.000000") "Undefined" "MultiplyWithRoot" 0 0)
    (if (== (Variables|Default|GetCut) 2)
      (Actor|DestroyActor))))

(event OnComponentEndOverlap(Box)
  (params (OverlappedComponent :type Primitive%20Component%20Object%20Reference) (OtherActor :type Actor%20Object%20Reference) (OtherComp :type Primitive%20Component%20Object%20Reference) (OtherBodyIndex :type Integer))
  (Utilities|FlowControl|Delay 0.5)
  (Variables|Default|SetDelay true))

(fn ConstructionScript)