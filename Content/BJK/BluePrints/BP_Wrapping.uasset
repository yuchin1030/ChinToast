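; Food assembly actor that stacks overlapping ingredients and checks them against a recipe.
; The first five overlaps on CheckF snap to mesh sockets A to E in turn, each slot firing once via DoOnce.
; CheckFood casts each actor to its ingredient class and logs its name in MakingFood.
; After the fifth, CheckRecipe compares that order with the level's Recipe actor and only prints results, using entry zero as the success text.
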(event OnComponentBeginOverlap(CheckF)
  (params (OverlappedComponent :type Primitive%20Component%20Object%20Reference) (OtherActor :type Actor%20Object%20Reference) (OtherComp :type Primitive%20Component%20Object%20Reference) (OtherBodyIndex :type Integer) (bFromSweep :type Boolean) (SweepResult :type Hit%20Result%20Structure%20%28by%20ref%29))
  (bind _staticmesh (Variables|Default|GetStaticMesh))
  (bind _staticmesh_2 (Variables|Default|GetStaticMesh))
  (switch int (Variables|Default|GetisAttach)
    (:0
      (Utilities|FlowControl|DoOnce false
        (:Completed
          (Transformation|AttachComponentToComponent (Variables|/Script/Engine.Actor|GetRootComponent OtherActor) (Variables|Default|GetStaticMesh) "A" "SnapToTarget" "SnapToTarget" "SnapToTarget" true)
          (bind _result (Math|Integer|IncrementInt (Variables|Default|GetisAttach))
            (:%20%20
              (bind _output_get (Variables|Default|SetisAttach _result))
              (Development|PrintString (Utilities|String|ToString(Integer) _output_get))
              (CallFunction|CheckFood OtherActor))))))
    (:1
      (Utilities|FlowControl|DoOnce false
        (:Completed
          (Transformation|AttachComponentToComponent (Variables|/Script/Engine.Actor|GetRootComponent OtherActor) _staticmesh_2 "B" "SnapToTarget" "SnapToTarget" "SnapToTarget" true)
          (bind _result_2 (Math|Integer|IncrementInt (Variables|Default|GetisAttach))
            (:%20%20
              (bind _output_get_2 (Variables|Default|SetisAttach _result_2))
              (Development|PrintString (Utilities|String|ToString(Integer) _output_get_2))
              (CallFunction|CheckFood OtherActor))))))
    (:2
      (Utilities|FlowControl|DoOnce false
        (:Completed
          (Transformation|AttachComponentToComponent (Variables|/Script/Engine.Actor|GetRootComponent OtherActor) _staticmesh_2 "C" "SnapToTarget" "SnapToTarget" "SnapToTarget" true)
          (bind _result_3 (Math|Integer|IncrementInt (Variables|Default|GetisAttach))
            (:%20%20
              (bind _output_get_3 (Variables|Default|SetisAttach _result_3))
              (CallFunction|CheckFood OtherActor)
              (Development|PrintString (Utilities|String|ToString(Integer) _output_get_3)))))))
    (:3
      (Utilities|FlowControl|DoOnce false
        (:Completed
          (Transformation|AttachComponentToComponent (Variables|/Script/Engine.Actor|GetRootComponent OtherActor) _staticmesh "D" "SnapToTarget" "SnapToTarget" "SnapToTarget" true)
          (bind _result_4 (Math|Integer|IncrementInt (Variables|Default|GetisAttach))
            (:%20%20
              (bind _output_get_4 (Variables|Default|SetisAttach _result_4))
              (CallFunction|CheckFood OtherActor)
              (Development|PrintString (Utilities|String|ToString(Integer) _output_get_4)))))))
    (:4
      (Utilities|FlowControl|DoOnce false
        (:Completed
          (Transformation|AttachComponentToComponent (Variables|/Script/Engine.Actor|GetRootComponent OtherActor) _staticmesh "E" "SnapToTarget" "SnapToTarget" "SnapToTarget" true)
          (bind _result_5 (Math|Integer|IncrementInt (Variables|Default|GetisAttach))
            (:%20%20
              (bind _output_get_5 (Variables|Default|SetisAttach _result_5))
              (CallFunction|CheckFood OtherActor)
              (Development|PrintString (Utilities|String|ToString(Integer) _output_get_5))
              (for _array_element (Variables|Default|GetMakingFood)
                (Development|PrintString _array_element))
              (Development|PrintString (Utilities|String|ToString(Integer) (Utilities|Array|Length (Variables|Default|GetMakingFood))))
              (CallFunction|CheckRecipe))))))))

(event Custom|CheckRecipe
  (bind _recipevar (Variables|Default|GetRecipeVar))
  (bind _makedrecipe (Variables|/Script/ChinToast.ChinToastRecipe|GetmakedRecipe _recipevar))
  (bind _index (Utilities|FlowControl|ForLoopwithBreak 1 5 :!label _label)
    (:LoopBody
      (if (Utilities|Enum|Equal(Enum) (Utilities|Array|Get(acopy) _makedrecipe (Variables|Default|GetIndex)) (Utilities|Array|Get(acopy) (Variables|Default|GetMakingFood) (- (Variables|Default|GetIndex) 1)))
        (bind _result (Math|Integer|IncrementInt _index)
          (:%20%20
            (bind _output_get (Variables|Default|SetIndex _result))
            (Development|PrintString (Utilities|String|ToString(Integer) _output_get))))
        (else
          (Development|PrintString "false")
          (Variables|Default|Setsuccess false)
          (goto _label Break))))
    (:Completed
      (if (Variables|Default|Getsuccess)
        (Development|PrintString (Utilities|Array|Get(acopy) _makedrecipe))))))

(event EventBeginPlay
  (bind _outactors (Actor|GetAllActorsOfClass "/Game/KSW/Recipe.Recipe_C"))
  (Variables|Default|SetRecipeVar (Utilities|Array|Get(acopy) _outactors)))

(fn ConstructionScript)

(fn CheckFood
  (params (NewParam :type Actor%20Object%20Reference))
  (bind _asbp_bread (Utilities|Casting|CastToBP_Bread NewParam)
    (:then
      (Physics|SetPhysicsLinearVelocity (Variables|/Game/BJK/BluePrints/Food/BP_Bread.BP_Bread_C|GetStaticMesh _asbp_bread) "0, 0, 0" false "None")
      (Utilities|Array|Add (Variables|Default|GetMakingFood) "Bread"))
    (:CastFailed
      (Utilities|Casting|CastToBP_Tomato NewParam
        (:then
          (Utilities|Array|Add (Variables|Default|GetMakingFood) "Tomato"))
        (:CastFailed
          (Utilities|Casting|CastToBP_Ham NewParam
            (:then
              (Utilities|Array|Add (Variables|Default|GetMakingFood) "Hams"))
            (:CastFailed
              (Utilities|Casting|CastToBP_Chesse NewParam
                (:then
                  (Utilities|Array|Add (Variables|Default|GetMakingFood) "Chesse"))
                (:CastFailed
                  (Utilities|Casting|CastToBP_Lettuce NewParam)
                  (Utilities|Array|Add (Variables|Default|GetMakingFood) "Lettuce"))))))))))