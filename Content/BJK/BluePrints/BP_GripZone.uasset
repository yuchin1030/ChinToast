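; BP_GripZone is a box trigger that flags the test player's IsTomato state while an overlap lasts, apparently as a grip zone.
; Begin and end overlap compare the other actor to HandLeft on a stored player reference, which these graphs never assign.
; On a match, they cast that actor to BP_TestPlayer and set IsTomato true on entry, false on exit.
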(event OnComponentEndOverlap(Box)
  (params (OverlappedComponent :type Primitive%20Component%20Object%20Reference) (OtherActor :type Actor%20Object%20Reference) (OtherComp :type Primitive%20Component%20Object%20Reference) (OtherBodyIndex :type Integer))
  (if (== OtherActor (Variables|/Game/BJK/BluePrints/BP_TestPlayer.BP_TestPlayer_C|GetHandLeft (Variables|Default|GetAs%20BP%20Test%20Player)))
    (bind _asbp_test_player (Utilities|Casting|CastToBP_TestPlayer OtherActor))
    (Variables|/Game/BJK/BluePrints/BP_TestPlayer.BP_TestPlayer_C|SetisTomato _asbp_test_player false)))

(event OnComponentBeginOverlap(Box)
  (params (OverlappedComponent :type Primitive%20Component%20Object%20Reference) (OtherActor :type Actor%20Object%20Reference) (OtherComp :type Primitive%20Component%20Object%20Reference) (OtherBodyIndex :type Integer) (bFromSweep :type Boolean) (SweepResult :type Hit%20Result%20Structure%20%28by%20ref%29))
  (if (== OtherActor (Variables|/Game/BJK/BluePrints/BP_TestPlayer.BP_TestPlayer_C|GetHandLeft (Variables|Default|GetAs%20BP%20Test%20Player)))
    (bind _asbp_test_player (Utilities|Casting|CastToBP_TestPlayer OtherActor))
    (Variables|/Game/BJK/BluePrints/BP_TestPlayer.BP_TestPlayer_C|SetisTomato _asbp_test_player true)))

(fn ConstructionScript)