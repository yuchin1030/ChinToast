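; BP_Setting is a tray station where a wrapped toast is delivered and scored.
; The first overlap on BoxingCol fires a DoOnce that casts to BP_Wrapping, turns off its physics, calls DestroyGrab and snaps it to the tray socket.
; If the wrapping has not failed, it adds score, spawns a floating score actor, removes the food and box, and sets IsGameOver.
; The ButtonCol overlap is empty.
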(event OnComponentBeginOverlap(BoxingCol)
  (params (OverlappedComponent :type Primitive%20Component%20Object%20Reference) (OtherActor :type Actor%20Object%20Reference) (OtherComp :type Primitive%20Component%20Object%20Reference) (OtherBodyIndex :type Integer) (bFromSweep :type Boolean) (SweepResult :type Hit%20Result%20Structure%20%28by%20ref%29))
  (bind _returnvalue (Transformation|GetActorTransform))
  (Utilities|FlowControl|DoOnce false
    (:Completed
      (bind _asbp_wrapping (Utilities|Casting|CastToBP_Wrapping OtherActor))
      (Physics|SetSimulatePhysics (Variables|/Game/BJK/BluePrints/BP_Wrapping.BP_Wrapping_C|GetStaticMesh _asbp_wrapping) false)
      (Default|DestroyGrab _asbp_wrapping)
      (Transformation|AttachComponentToComponent (Variables|/Script/Engine.Actor|GetRootComponent _asbp_wrapping) (Variables|Default|GetTray) "TaryS" "SnapToTarget" "SnapToTarget" "SnapToTarget" true)
      (if (not (Variables|/Game/BJK/BluePrints/BP_Wrapping.BP_Wrapping_C|Getfail _asbp_wrapping)) ; 토스트 재료들이 모두 알맞게 들어가면
        (bind _output_get (Variables|Default|SetScore (+ (Variables|Default|GetScore) 100)))
        (Game|SpawnActorfromClass "/Game/Yuchin/Blueprints/BP_SpawnedPlusScore.BP_SpawnedPlusScore_C" (Math|Transform|MakeTransform (+ (.location _returnvalue) "30.000000,0.000000,50.000000") (.rotation _returnvalue) "0.500000,0.500000,0.500000") "Undefined" "MultiplyWithRoot" 0 _output_get 0) ; 플러스되는 점수 UI 띄우기
        (Variables|Default|SetSum (+ (Variables|Default|GetSum) (Variables|Default|GetScore)))
        (Default|DestroyFoodandBox _asbp_wrapping) ; 쟁반에 올려지면 포장박스, 재료들 삭제
        (Variables|Default|SetisGameOver true)))))

(event OnComponentBeginOverlap(ButtonCol)
  (params (OverlappedComponent :type Primitive%20Component%20Object%20Reference) (OtherActor :type Actor%20Object%20Reference) (OtherComp :type Primitive%20Component%20Object%20Reference) (OtherBodyIndex :type Integer) (bFromSweep :type Boolean) (SweepResult :type Hit%20Result%20Structure%20%28by%20ref%29)))

(fn ConstructionScript)