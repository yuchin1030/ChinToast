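; Game countdown timer actor that ends the round by showing the final result and removing customers.
; Tick feeds a one-second Delay that counts Seconds and Minutes down, using the latent node as the timer.
; At zero it calls ShowFinalResult on the BP_SpawnFinalResult cached at BeginPlay, then destroys a BP_Customer and its root component.
; Nothing stops the countdown at zero, so this end step repeats every second.
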(event EventBeginPlay
  (bind _outactors (Actor|GetAllActorsOfClass "/Game/Yuchin/Blueprints/BP_SpawnFinalResult.BP_SpawnFinalResult_C"))
  (Variables|Default|SetSpawnFinalResultVar (Utilities|Array|Get(acopy) _outactors)))

(event EventTick
  (params (DeltaSeconds :type Float%20%28single-precision%29))
  (Utilities|FlowControl|Delay 1.0)
  (if (== (Variables|Default|GetSeconds) 0)
    (if (== (Variables|Default|GetMinutes) 0)
      (Default|ShowFinalResult (Variables|Default|GetSpawnFinalResultVar))
      (bind _returnvalue (Actor|GetActorOfClass "/Game/KSW/BP_Customer.BP_Customer_C"))
      (Utilities|IsValid _returnvalue
        (:Is%20Valid
          (Actor|DestroyActor _returnvalue)
          (Utilities|IsValid (Variables|/Script/Engine.Actor|GetRootComponent _returnvalue)
            (:Is%20Valid
              (Components|DestroyComponent (Variables|/Script/Engine.Actor|GetRootComponent _returnvalue))))))
      (else
        (Variables|Default|SetSeconds 59)
        (Variables|Default|SetMinutes (- (Variables|Default|GetMinutes) 1))))
    (else
      (Variables|Default|SetSeconds (- (Variables|Default|GetSeconds) 1)))))

(fn ConstructionScript)