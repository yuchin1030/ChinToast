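; BP_Toaster is a toaster actor that starts toasting or burning bread placed inside its Box trigger.
; On overlap, a BP_BreadBase is flagged as baking and a BP_Bread as burning, with a short named timer set to call MakeToast or MakeBurn on that bread.
; Leaving the box clears the flag but not the timer, so the delayed call still fires on the bread.
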(event OnComponentBeginOverlap(Box)
  (params (OverlappedComponent :type Primitive%20Component%20Object%20Reference) (OtherActor :type Actor%20Object%20Reference) (OtherComp :type Primitive%20Component%20Object%20Reference) (OtherBodyIndex :type Integer) (bFromSweep :type Boolean) (SweepResult :type Hit%20Result%20Structure%20%28by%20ref%29))
  (bind _asbp_bread_base (Utilities|Casting|CastToBP_BreadBase OtherActor)
    (:then
      (Variables|/Game/BJK/BluePrints/Food/BP_BreadBase.BP_BreadBase_C|SetisBaking _asbp_bread_base true)
      (Utilities|Time|SetTimerbyFunctionName _asbp_bread_base "MakeToast" 3.0))
    (:CastFailed
      (bind _asbp_bread (Utilities|Casting|CastToBP_Bread OtherActor))
      (Variables|/Game/BJK/BluePrints/Food/BP_Bread.BP_Bread_C|SetisBurning _asbp_bread true)
      (Utilities|Time|SetTimerbyFunctionName _asbp_bread "MakeBurn" 3.0))))

(event OnComponentEndOverlap(Box)
  (params (OverlappedComponent :type Primitive%20Component%20Object%20Reference) (OtherActor :type Actor%20Object%20Reference) (OtherComp :type Primitive%20Component%20Object%20Reference) (OtherBodyIndex :type Integer))
  (bind _asbp_bread_base (Utilities|Casting|CastToBP_BreadBase OtherActor)
    (:then
      (Variables|/Game/BJK/BluePrints/Food/BP_BreadBase.BP_BreadBase_C|SetisBaking _asbp_bread_base false))
    (:CastFailed
      (bind _asbp_bread (Utilities|Casting|CastToBP_Bread OtherActor))
      (Variables|/Game/BJK/BluePrints/Food/BP_Bread.BP_Bread_C|SetisBurning _asbp_bread false))))

(event EventBeginPlay)

(event Collision|EventActorBeginOverlap
  (params (OtherActor :type Actor%20Object%20Reference)))

(event EventTick
  (params (DeltaSeconds :type Float%20%28single-precision%29)))

(fn ConstructionScript)